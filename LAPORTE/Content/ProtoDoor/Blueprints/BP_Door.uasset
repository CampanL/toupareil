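; BP_Door is an interactable door that swings open or closed around its yaw when the player interacts.
; Interact calls CallMoveToDoor if the first-person character is not at the door; otherwise it toggles between OpenDoor and CloseDoor, ignoring input mid-swing.
; Timeline updates serve as tick loops, rotating the Scene component by RotationSpeed and stored Tick delta time, then snapping at OpenAngle or zero and stopping.
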(event `self.ReceiveTick`
  (params (DeltaSeconds :type "Float (single-precision)"))
  (`parent.ReceiveTick` DeltaSeconds)
  (set `self.StoredDeltaTime` DeltaSeconds))

(event `CloseDoor`
  (bind _scene (`self.Scene`))
  (bind _storeddeltatime (`self.StoredDeltaTime`))
  (bind _returnvalue (* _storeddeltatime (`self.RotationSpeed`)))
  (bind (_relativerotation_roll _relativerotation_pitch _relativerotation_yaw) (`KismetMathLibrary.BreakRotator` (`SceneComponent.RelativeRotation` _scene)))
  ;[1 1 1] Close door
  (`Timeline|Timeline_0` :!label _label
    (:`Update`
      (if (< _storeddeltatime 0.0)
        (`SceneComponent.K2_AddRelativeRotation` _scene (`KismetMathLibrary.MakeRotator` 0.0 0.0 _returnvalue) false false)
        (if (> _relativerotation_yaw 0.0)
          (`SceneComponent.K2_SetRelativeRotation` _scene (`KismetMathLibrary.MakeRotator` 0.0) false false :!label _label_2)
          (set `self.open` false)
          (set `self.Interacted` false)
          (`KismetSystemLibrary.PrintString` "Door closed")
          (goto _label :!via `Stop`))
        (else
          (`SceneComponent.K2_AddRelativeRotation` _scene (`KismetMathLibrary.MakeRotator` 0.0 0.0 (* _returnvalue -1.0)) false false)
          (if (< _relativerotation_yaw 0.0)
            (goto _label_2)))))))

(event `OpenDoor`
  (bind _scene (`self.Scene`))
  (bind _storeddeltatime (`self.StoredDeltaTime`))
  (bind _openangle (`self.OpenAngle`))
  (bind _returnvalue (* _storeddeltatime (`self.RotationSpeed`)))
  (bind (_relativerotation_roll _relativerotation_pitch _relativerotation_yaw) (`KismetMathLibrary.BreakRotator` (`SceneComponent.RelativeRotation` _scene)))
  ;[1 1 1] Open the door
  (`Timeline|Timeline` :!label _label_3
    (:`Update`
      (if (> _storeddeltatime 0.0)
        (`SceneComponent.K2_AddRelativeRotation` _scene (`KismetMathLibrary.MakeRotator` 0.0 0.0 _returnvalue) false false)
        (if (> _relativerotation_yaw _openangle)
          (`SceneComponent.K2_SetRelativeRotation` _scene (`KismetMathLibrary.MakeRotator` 0.0 0.0 _openangle) false false :!label _label_4)
          (set `self.open` true)
          (set `self.Interacted` false)
          (`KismetSystemLibrary.PrintString` "Door opened")
          (goto _label_3 :!via `Stop`))
        (else
          (`SceneComponent.K2_AddRelativeRotation` _scene (`KismetMathLibrary.MakeRotator` 0.0 0.0 (* _returnvalue -1.0)) false false)
          (if (< _relativerotation_yaw _openangle)
            (goto _label_4)))))))

(event `self.ReceiveBeginPlay`
  (`parent.ReceiveBeginPlay`)
  (bind _asbp_first_person_character (cast `/Game/FirstPerson/Blueprints/BP_FirstPersonCharacter` (`GameplayStatics.GetPlayerCharacter` 0)))
  (set `self.PlayerRef` _asbp_first_person_character))

(fn `Interact`
  (`parent.Interact`)
  (if (`/Game/FirstPerson/Blueprints/BP_FirstPersonCharacter.IsAtDoor` (`self.PlayerRef`))
    (if (not (`self.Interacted`))
      (set `self.Interacted` true)
      (if (`self.open`)
        (`self.CloseDoor`)
        (else
          (`self.OpenDoor`))))
    (else
      (`self.MoveToDoor`))))

(fn `UserConstructionScript`
  (`parent.UserConstructionScript`))