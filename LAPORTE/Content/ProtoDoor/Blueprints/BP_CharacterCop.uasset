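; BP_CharacterCop is the cop variant of a door visitor that knocks, rings the doorbell and waits.
; On BeginPlay it applies a random cop material and sets its doorbell count and open/closed door texts.
; It then reads the suspicion state (Safe, Conflict or Madness) from BP_HouseSuspicionEvents to pick per-state suspicion values, knock count and wait time from arrays.
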(event `self.ReceiveBeginPlay`
  (set `self.MaterialsRandom` (`self.Materials Random Cop`))
  (`self.SetRandomMat`)
  (set `self.TimesHittingDoorbell` 3)
  (set `self.TextOpen` (`self.TextOpenCop`))
  (set `self.TextClosed` (`self.TextCloseCop`))
  (bind _returnvalue (`GameplayStatics.GetActorOfClass` "/Game/ProtoDoor/Blueprints/BP_HouseSuspicionEvents.BP_HouseSuspicionEvents_C"))
  (switch `/Game/ProtoDoor/Blueprints/E_SuspicionState` (`/Game/ProtoDoor/Blueprints/BP_HouseSuspicionEvents.SuspictionState` _returnvalue)
    (:`NewEnumerator0`
      (set `self.SuspicionOpenDoorValue` (`|GetArrayItem` (`self.SuspicionOpen`)))
      (set `self.SuspicionCloseDoorValue` (`|GetArrayItem` (`self.SuspicionClose`)))
      (set `self.TimesKnocking` (`|GetArrayItem` (`self.KnockTimes`)))
      (set `self.TimeToStayAtDoor` (`|GetArrayItem` (`self.TimeWaitingAtDoor`))))
    (:`NewEnumerator1`
      (set `self.SuspicionOpenDoorValue` (`|GetArrayItem` (`self.SuspicionOpen`) 1))
      (set `self.SuspicionCloseDoorValue` (`|GetArrayItem` (`self.SuspicionClose`) 1))
      (set `self.TimesKnocking` (`|GetArrayItem` (`self.KnockTimes`) 1))
      (set `self.TimeToStayAtDoor` (`|GetArrayItem` (`self.TimeWaitingAtDoor`) 1)))
    (:`NewEnumerator2`
      (set `self.SuspicionOpenDoorValue` (`|GetArrayItem` (`self.SuspicionOpen`) 2))
      (set `self.SuspicionCloseDoorValue` (`|GetArrayItem` (`self.SuspicionClose`) 2))
      (set `self.TimesKnocking` (`|GetArrayItem` (`self.KnockTimes`) 2))
      (set `self.TimeToStayAtDoor` (`|GetArrayItem` (`self.TimeWaitingAtDoor`) 2)))))

(fn `UserConstructionScript`
  (`parent.UserConstructionScript`))