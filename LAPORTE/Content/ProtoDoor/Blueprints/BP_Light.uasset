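; BP_Light is a point light actor in ProtoDoor that switches between three color states: safe, conflict and madness.
; At BeginPlay it stores the point light's initial color as the safe color, so that state restores the original look.
; One function per state applies the stored color to the light; nothing in this Blueprint calls them.
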(event `self.ReceiveBeginPlay`
  (set `self.ColorSafe` (`KismetMathLibrary.Conv_LinearColorToColor` (`LightComponentBase.GetLightColor` (`self.PointLight`)))))

(fn `SetColorConflict`
  (`LightComponent.SetLightColor` (`self.PointLight`) (`KismetMathLibrary.Conv_ColorToLinearColor` (`self.ColorConflict`)) true))

(fn `SetColorMadness`
  (`LightComponent.SetLightColor` (`self.PointLight`) (`KismetMathLibrary.Conv_ColorToLinearColor` (`self.ColorMadness`)) true))

(fn `SetColorSafe`
  (`LightComponent.SetLightColor` (`self.PointLight`) (`KismetMathLibrary.Conv_ColorToLinearColor` (`self.ColorSafe`)) true))

(fn `UserConstructionScript`)