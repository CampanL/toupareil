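; Delivery courier variant of the character event pawn, a door visitor who arrives holding a box.
; On BeginPlay it sets delivery text, plays the box montage and picks suspicion values, knock count and wait time from per-state arrays using BP_HouseSuspicionEvents' Safe, Conflict or Madness state.
; Opening the door clears HoldingBox after a short delay, so Tick hides the parcel once and switches to idle.
; The door-not-opened handler is empty.
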(event `self.ReceiveBeginPlay`
  (add `self.OnDoorOpened` (delegate `DeliveryOpen`))
  (add `self.OnDoorNotOpened` (delegate `DeliveryClose`))
  (set `self.TextOpen` (`self.TextOpenDelivery`))
  (set `self.TextClosed` (`self.TextCloseDelivery`))
  (set `self.HoldingBox` true)
  (`self.PlayAnimMontage` "/Game/ProtoDoor/Basti/Animations/Anim_BoxMontage.Anim_BoxMontage")
  (bind _returnvalue (`GameplayStatics.GetActorOfClass` "/Game/ProtoDoor/Blueprints/BP_HouseSuspicionEvents.BP_HouseSuspicionEvents_C"))
  (switch `/Game/ProtoDoor/Blueprints/E_SuspicionState` (`/Game/ProtoDoor/Blueprints/BP_HouseSuspicionEvents.SuspictionState` _returnvalue)
    (:`NewEnumerator0`
      (set `self.SuspicionOpenDoorValue` (`|GetArrayItem` (`self.SuspicionOpen`)))
      (set `self.SuspicionCloseDoorValue` (`|GetArrayItem` (`self.SuspicionClose`)))
      (set `self.TimesKnocking` (`|GetArrayItem` (`self.KnockTimes`)))
      (set `self.TimeToStayAtDoor` (`|GetArrayItem` (`self.TimeWaitingAtDoor`))))
    (:`NewEnumerator1`
      (set `self.SuspicionOpenDoorValue` (`|GetArrayItem` (`self.SuspicionOpen`) 1))
      (set `self.SuspicionCloseDoorValue` (`|GetArrayItem` (`self.SuspicionClose`) 1))
      (set `self.TimesKnocking` (`|GetArrayItem` (`self.KnockTimes`) 1))
      (set `self.TimeToStayAtDoor` (`|GetArrayItem` (`self.TimeWaitingAtDoor`) 1)))
    (:`NewEnumerator2`
      (set `self.SuspicionOpenDoorValue` (`|GetArrayItem` (`self.SuspicionOpen`) 2))
      (set `self.SuspicionCloseDoorValue` (`|GetArrayItem` (`self.SuspicionClose`) 2))
      (set `self.TimesKnocking` (`|GetArrayItem` (`self.KnockTimes`) 2))
      (set `self.TimeToStayAtDoor` (`|GetArrayItem` (`self.TimeWaitingAtDoor`) 2)))))

(event `DeliveryOpen` :!signature `self.OnDoorOpened`
  (params (CharacterEventRef :type "/Game/ProtoDoor/Blueprints/BP_CharacterEventPawn Object Reference") (Suspicion :type "Float (double-precision)"))
  (`KismetSystemLibrary.Delay` 1.0)
  (set `self.HoldingBox` false))

(event `self.ReceiveTick`
  (params (DeltaSeconds :type "Float (single-precision)"))
  (`parent.ReceiveTick` DeltaSeconds)
  (if (not (`self.HoldingBox`))
    (`/Engine/EditorBlueprintResources/StandardMacros.DoOnce` false
      (:`Completed`
        (`SceneComponent.SetVisibility` (`self.Colis`) false false)
        (`self.PlayAnimMontage` "/Game/ProtoDoor/Basti/Animations/Idle_Anim_mixamo_com_Montage.Idle_Anim_mixamo_com_Montage")))))

(event `DeliveryClose` :!signature `self.OnDoorNotOpened`
  (params (CharacterEventRef :type "/Game/ProtoDoor/Blueprints/BP_CharacterEventPawn Object Reference") (SuspicionValue :type "Float (double-precision)")))

(fn `UserConstructionScript`
  (`parent.UserConstructionScript`)
  (set `self.TimesHittingDoorbell` 1)
  (set `self.TimesKnocking` 2))