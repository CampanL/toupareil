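; BP_DigitalClock is an actor that shows an hour-only digital clock on a TextRender, wrapping to zero after 23.
; BeginPlay stores the configured seconds per hour, shows the starting hour with a leading zero and looks up BP_Door without using the result.
; Tick counts down by delta time, then increments the hour, rewrites the text with conditional zero-padding and restarts the countdown.
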(event `self.ReceiveBeginPlay`
  (`GameplayStatics.GetActorOfClass` "/Game/ProtoDoor/Blueprints/BP_Door.BP_Door_C")
  (set `self.InitSecondsToWait` (`self.SecondsToWaitForHour`))
  (`TextRenderComponent.K2_SetText` (`self.TextRender`) (`KismetTextLibrary.Conv_StringToText` (`KismetStringLibrary.Concat_StrStr` "0" (`KismetStringLibrary.Conv_IntToString` (`self.CustomTimeValueToDisplay`)) ":00"))))

(event `self.ReceiveTick`
  (params (DeltaSeconds :type "Float (single-precision)"))
  (bind _customtimevaluetodisplay (`self.CustomTimeValueToDisplay`))
  (bind _initsecondstowait (`self.InitSecondsToWait`))
  (if true
    (bind _output_get (set `self.SecondsToWaitForHour` (- (`self.SecondsToWaitForHour`) DeltaSeconds)))
    (if (<= _output_get 0.0)
      (bind _result (`/Engine/EditorBlueprintResources/StandardMacros.IncrementInt` _customtimevaluetodisplay)
        (:`  `
          (if (> _customtimevaluetodisplay 23)
            (set `self.CustomTimeValueToDisplay` 0))
          (if (> _result 9)
            (`TextRenderComponent.K2_SetText` (`self.TextRender`) (`KismetTextLibrary.Conv_StringToText` (`KismetStringLibrary.Concat_StrStr` (`KismetStringLibrary.Conv_IntToString` _customtimevaluetodisplay) ":00")))
            (set `self.SecondsToWaitForHour` _initsecondstowait)
            (else
              (`TextRenderComponent.K2_SetText` (`self.TextRender`) (`KismetTextLibrary.Conv_StringToText` (`KismetStringLibrary.Concat_StrStr` "0" (`KismetStringLibrary.Conv_IntToString` _customtimevaluetodisplay) ":00")))
              (set `self.SecondsToWaitForHour` _initsecondstowait))))))))

(fn `UserConstructionScript`)