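; BP_CharacterEventPawn is an AI-moved pawn that walks to a given target, apparently a door, and makes repeated sounds while waiting there.
; MoveToTarget runs AIMoveTo on the target's X and Y, then sets IsWaitingAtDoor on success.
; While that flag is set, a random-length Delay on Tick acts as a repeat timer, replaying the audio at a random pitch.
; Nothing in this Blueprint clears the flag.
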(event `MoveToTarget`
  (params (Target :type "Vector Structure"))
  (`|AIMoveTo` self (`KismetMathLibrary.MakeVector` (.x Target) (.y Target)) null
    (:`OnSuccess`
      (set `self.isWaitingAtDoor` true))))

(event `self.ReceiveTick`
  (params (DeltaSeconds :type "Float (single-precision)"))
  (bind _audio (`self.Audio`))
  (if (`self.isWaitingAtDoor`)
    (`KismetSystemLibrary.Delay` (`KismetMathLibrary.RandomFloatInRange` 2.5 4.0))
    (`AudioComponent.SetPitchMultiplier` _audio (`KismetMathLibrary.RandomFloatInRange` 0.5 1.25))
    (`AudioComponent.Play` _audio 0.0)))

(fn `UserConstructionScript`)