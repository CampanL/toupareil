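; BP_HouseSuspicionEvents switches the house lighting between safe, conflict and madness states based on the first-person player's suspicion value.
; Tick compares that value against conflict and madness thresholds, using DoOnce gates reset by neighboring bands to fire on band changes.
; Each change recolors every BP_Light, updates the suspicion state and prints a debug message.
; A WasMadness flag, set in madness and cleared in safe, is passed to the conflict color change.
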(event `self.ReceiveBeginPlay`
  (bind _asbp_first_person_character (cast `/Game/FirstPerson/Blueprints/BP_FirstPersonCharacter` (`GameplayStatics.GetPlayerCharacter` 0)))
  (set `self.PlayerRef` _asbp_first_person_character))

(event `self.ReceiveTick`
  (params (DeltaSeconds :type "Float (single-precision)"))
  (bind _suspicionvalue (`/Game/FirstPerson/Blueprints/BP_FirstPersonCharacter.SuspicionValue` (`self.PlayerRef`)))
  (if (< _suspicionvalue (`self.ConflictThreshold`))
    ;[1 1 1] SafeTime
    (`|ExecutionSequence`
      (:`then_0`
        (`/Engine/EditorBlueprintResources/StandardMacros.DoOnce` false :!label _label
          (:`Completed`
            (bind _outactors (`GameplayStatics.GetAllActorsOfClass` "/Game/ProtoDoor/Blueprints/BP_Light.BP_Light_C"))
            (for _array_element _outactors
              (`/Game/ProtoDoor/Blueprints/BP_Light.SetColorSafe` _array_element))
            (`KismetSystemLibrary.PrintString` "ChangedLightsToSafe")
            (set `self.WasMadness` false)
            (set `self.SuspictionState` "NewEnumerator0"))))
      (:`then_1`
        (goto _label_2 :!via `Reset`)))
    (elif (< _suspicionvalue (`self.MadnessThreshold`))
      ;[1 1 1] ConflictTime
      (`|ExecutionSequence`
        (:`then_0`
          (`/Engine/EditorBlueprintResources/StandardMacros.DoOnce` false :!label _label_2
            (:`Completed`
              (bind _outactors_2 (`GameplayStatics.GetAllActorsOfClass` "/Game/ProtoDoor/Blueprints/BP_Light.BP_Light_C"))
              (for _array_element_2 _outactors_2
                (`/Game/ProtoDoor/Blueprints/BP_Light.SetColorConflict` _array_element_2 (`self.WasMadness`)))
              (`KismetSystemLibrary.PrintString` "ChangedLightsToConflict")
              (set `self.SuspictionState` "NewEnumerator1"))))
        (:`then_1`
          (goto _label :!via `Reset`))
        (:`then_2`
          (goto _label_3 :!via `Reset`)))
      (else
        ;[1 1 1] MadnessTime
        (`|ExecutionSequence`
          (:`then_0`
            (`/Engine/EditorBlueprintResources/StandardMacros.DoOnce` false :!label _label_3
              (:`Completed`
                (bind _outactors_3 (`GameplayStatics.GetAllActorsOfClass` "/Game/ProtoDoor/Blueprints/BP_Light.BP_Light_C"))
                (for _array_element_3 _outactors_3
                  (`/Game/ProtoDoor/Blueprints/BP_Light.SetColorMadness` _array_element_3))
                (`KismetSystemLibrary.PrintString` "ChangedLightsToMadness")
                (set `self.WasMadness` true)
                (set `self.SuspictionState` "NewEnumerator2"))))
          (:`then_1`
            (goto _label_2 :!via `Reset`)))))))

(fn `UserConstructionScript`)