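; BP_CharacterPaparazzi is an AI-moved paparazzi character that fires camera flashes when a door opens, then leaves.
; MoveToTarget starts movement to a given location, caches a BP_Door and arms a wait flag, with an eight-second timeout that also sends it away.
; Tick polls the door's Open state, then double-fires its child BP_CameraFlash after a short delay and moves to DispawnPoint, destroying itself on arrival.
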(event `MoveToTarget`
  (params (`Location To Move To` :type "Vector Structure"))
  (`|AIMoveTo` self (`KismetMathLibrary.MakeVector` (.x `Location To Move To`) (.y `Location To Move To`)) null
    (:`then`
      (set `self.WaitForDoorToOpen` true)
      (bind _returnvalue (`GameplayStatics.GetActorOfClass` "/Game/Blueprints/BP_Door.BP_Door_C"))
      (`KismetSystemLibrary.Delay` 8.0)
      (`|AIMoveTo` self (`KismetMathLibrary.MakeVector` (.x (`self.DispawnPoint`)) (.y (`self.DispawnPoint`))) null
        (:`OnSuccess`
          (`self.K2_DestroyActor`))))))

(event `self.ReceiveTick`
  (params (DeltaSeconds :type "Float (single-precision)"))
  (if (`self.WaitForDoorToOpen`)
    (if (`/Game/Blueprints/BP_Door.open` (stale `MoveToTarget` _returnvalue))
      (set `self.WaitForDoorToOpen` false)
      (`KismetSystemLibrary.Delay` 0.8)
      (bind _asbp_camera_flash (cast `/Game/ProtoDoor/Blueprints/BP_CameraFlash` (`ChildActorComponent.ChildActor` (`self.ChildActor`))))
      (`/Game/ProtoDoor/Blueprints/BP_CameraFlash.Flash` _asbp_camera_flash)
      (`KismetSystemLibrary.Delay` 0.2)
      (`/Game/ProtoDoor/Blueprints/BP_CameraFlash.Flash` _asbp_camera_flash)
      (`|AIMoveTo` self (`KismetMathLibrary.MakeVector` (.x (`self.DispawnPoint`)) (.y (`self.DispawnPoint`))) null
        (:`OnSuccess`
          (`self.K2_DestroyActor`))))))

(fn `UserConstructionScript`)