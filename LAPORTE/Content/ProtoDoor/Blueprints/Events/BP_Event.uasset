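; BP_Event is an event actor for the ProtoDoor prototype that changes suspicion depending on whether the event finishes or its door is ignored.
; EventFinished flags a valid linked EventToAffect as InfluencedByEvent, chaining events together.
; If influenced by another event or TV, finishing applies SuspicionDebuff and ignoring applies SuspicionBuff; otherwise the two are swapped.
; Both outcomes feed CallAddToSuspicion, while the event graph holds only disabled stubs.
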(fn `DoorIgnored`
  (if (or (`self.InfluencedByEvent`) (`self.InfluencedByTV`))
    (`self.AddToSuspicion` (`self.SuspicionBuff`))
    (else
      (`self.AddToSuspicion` (`self.SuspicionDebuff`)))))

(fn `EventFinished`
  (bind _eventtoaffect (`self.EventToAffect`))
  (`/Engine/EditorBlueprintResources/StandardMacros.IsValid` _eventtoaffect
    (:`Is Valid`
      (set `/Game/ProtoDoor/Blueprints/Events/BP_Event.InfluencedByEvent` true _eventtoaffect))
    (:`Is Not Valid`
      _))
  (if (or (`self.InfluencedByEvent`) (`self.InfluencedByTV`))
    (`self.AddToSuspicion` (`self.SuspicionDebuff`))
    (else
      (`self.AddToSuspicion` (`self.SuspicionBuff`)))))

(fn `UserConstructionScript`)