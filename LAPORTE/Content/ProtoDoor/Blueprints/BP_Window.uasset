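; BP_Window is a window actor that blurs its material as the player's suspicion rises.
; It caches the first-person character on BeginPlay and polls its SuspicionValue every Tick.
; While BlurFactor is below a tenth of that value, it recalculates the factor from suspicion and pushes it to the Cube's material scalar parameter, with no path to lower it.
; The construction script applies the initial value.
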(event `self.ReceiveBeginPlay`
  (bind _asbp_first_person_character (cast `/Game/FirstPerson/Blueprints/BP_FirstPersonCharacter` (`GameplayStatics.GetPlayerCharacter` 0)))
  (set `self.PlayerRef` _asbp_first_person_character))

(event `self.ReceiveTick`
  (params (DeltaSeconds :type "Float (single-precision)"))
  (bind _suspicionvalue (`/Game/FirstPerson/Blueprints/BP_FirstPersonCharacter.SuspicionValue` (`self.PlayerRef`)))
  (if (< (`self.BlurFactor`) (/ _suspicionvalue 10.0))
    (bind _output_get (set `self.BlurFactor` (* _suspicionvalue (+ (`self.BlurFactor`) 0.095))))
    (`MeshComponent.SetScalarParameterValueOnMaterials` (`self.Cube`) "BlurFactor" _output_get)))

(fn `UserConstructionScript`
  (`MeshComponent.SetScalarParameterValueOnMaterials` (`self.Cube`) "BlurFactor" (`self.BlurFactor`)))