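; BP_Door is an interactable door that swings open and closed by rotating its Scene component's yaw.
; Interact flags the door active and toggles its target, resetting the timer after completed swings; mid-swing, it can turn closing into opening but not the reverse.
; Tick lerps from the current yaw toward the open or closed angle, easing by elapsed time over OpenDoorTime, then prints the state and stops.
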(event `self.ReceiveTick`
  (params (DeltaSeconds :type "Float (single-precision)"))
  (bind _scene (`self.Scene`))
  (bind _opendoortime (`self.openDoorTime`))
  (bind _scene_2 (`self.Scene`))
  (bind _opendoortime_2 (`self.openDoorTime`))
  (`parent.ReceiveTick` DeltaSeconds)
  (if (`self.Interacted`)
    (if (`self.open`)
      (if (`self.timerReached`)
        (`KismetSystemLibrary.PrintString` "DoorOpened")
        (set `self.Interacted` false)
        (else
          (`SceneComponent.K2_SetRelativeRotation` _scene_2 (`KismetMathLibrary.MakeRotator` 0.0 0.0 (`KismetMathLibrary.Lerp` (.yaw (`SceneComponent.RelativeRotation` _scene_2)) -70.0 (/ (`self.timer`) _opendoortime_2))) false false)
          (bind _output_get (set `self.timer` (+ (`self.timer`) DeltaSeconds)))
          (`/Engine/EditorBlueprintResources/StandardMacros.CompareFloat` _output_get _opendoortime_2
            (:`>`
              _)
            (:`==`
              _))
          (set `self.timerReached` true)))
      (elif (`self.timerReached`)
        (`KismetSystemLibrary.PrintString` "DoorClosed")
        (set `self.Interacted` false)
        (else
          (`SceneComponent.K2_SetRelativeRotation` _scene (`KismetMathLibrary.MakeRotator` 0.0 0.0 (`KismetMathLibrary.Lerp` (.yaw (`SceneComponent.RelativeRotation` _scene)) 0.0 (/ (`self.timer`) _opendoortime))) false false)
          (bind _output_get_2 (set `self.timer` (+ (`self.timer`) DeltaSeconds)))
          (`/Engine/EditorBlueprintResources/StandardMacros.CompareFloat` _output_get_2 _opendoortime
            (:`>`
              _)
            (:`==`
              _))
          (set `self.timerReached` true))))))

(fn `Interact`
  (bind _timerreached (`self.timerReached`))
  (`parent.Interact`)
  (set `self.Interacted` true)
  (if (`self.open`)
    (if _timerreached
      (set `self.open` false)
      (set `self.timerReached` false)
      (set `self.timer` 0.0))
    (elif _timerreached
      (set `self.open` true)
      (set `self.timerReached` false)
      (set `self.timer` 0.0)
      (else
        (set `self.open` true)))))

(fn `UserConstructionScript`
  (`parent.UserConstructionScript`))